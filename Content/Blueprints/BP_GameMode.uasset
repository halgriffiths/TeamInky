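; BP_GameMode is a game mode Blueprint whose EndGame event closes out the running match.
; It makes each BP_PlayerController with a valid PreviousPawn repossess that pawn and destroys the pawn it was controlling.
; It then calls EndGame on the first FPSGameState and clears IsGameRunning.
; A camera blend to a BP_ViewPointHelper is left unconnected and never runs.
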(event `self.EndGame`
  (bind _outactors (`GameplayStatics.GetAllActorsOfClass` "/Game/Blueprints/BP_ViewPointHelper.BP_ViewPointHelper_C"))
  (bind _outactors_2 (`GameplayStatics.GetAllActorsOfClass` "/Game/Blueprints/BP_PlayerController.BP_PlayerController_C"))
  (for _array_element _outactors_2
    (bind _previouspawn (`FPSPlayerController.PreviousPawn` _array_element))
    (if (`KismetSystemLibrary.IsValid` _previouspawn)
      (bind _output_get (set `self.Aux` (`Controller.K2_GetPawn` _array_element)))
      (`Controller.Possess` _array_element _previouspawn)
      (`self.K2_DestroyActor` _output_get)))
  (bind _outactors_3 (`GameplayStatics.GetAllActorsOfClass` "/Script/FPSGame.FPSGameState"))
  (`FPSGameState.EndGame` (`|GetArrayItem` _outactors_3))
  (set `self.bIsGameRunning` false))

(fn `UserConstructionScript`)