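; BP_Player is the player Blueprint, tracking a temporary power-up state and a score.
; Capsule overlaps with BP_Ghost only print whether ghost or player was killed, based on HasActivePowerUp.
; Overlapping an FPSObjectiveActor sets that flag, and a timer by function name calls ResetPowerUp ten seconds later to clear it.
; OnScoreUpdated passes its increment to UpdateScore, which adds it to Score and prints the total.
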(event `self.ReceiveBeginPlay`
  (set `self.bHasActivePowerUp` false))

(event `self.CapsuleComponent.OnComponentBeginOverlap`
  (params (OverlappedComponent :type "PrimitiveComponent Object Reference") (OtherActor :type "Actor Object Reference") (OtherComp :type "PrimitiveComponent Object Reference") (OtherBodyIndex :type Integer) (bFromSweep :type Boolean) (SweepResult :type "HitResult Structure (by ref)"))
  (cast `/Game/Blueprints/BP_Ghost` OtherActor
    (:`then`
      (if (`self.bHasActivePowerUp`)
        (`KismetSystemLibrary.PrintText` "A Ghost has been killed by the Player")
        (else
          (`KismetSystemLibrary.PrintText` "The player has been killed by a Ghost!"))))
    (:`CastFailed`
      (cast `FPSObjectiveActor` OtherActor)
      (set `self.bHasActivePowerUp` true)
      (`KismetSystemLibrary.K2_SetTimer` null "ResetPowerUp" 10.0))))

(event `OnScoreUpdated`
  (params (`Score Increment` :type Integer))
  (`self.UpdateScore` `Score Increment`))

(fn `ResetPowerUp`
  (set `self.bHasActivePowerUp` false))

(fn `UpdateScore`
  (params (ScoreIncrement :type Integer))
  (bind _output_get (set `self.Score` (+ (`self.Score`) ScoreIncrement)))
  (`KismetSystemLibrary.PrintString` (`KismetStringLibrary.Concat_StrStr` "Current score is: " (`KismetStringLibrary.Conv_IntToString` _output_get))))

(fn `UserConstructionScript`)