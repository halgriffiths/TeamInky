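; Player controller that shows end-of-game screens and handles quit and admin reset keys.
; Mission-completed and game-over events create a WBP_GameOver widget with a success flag, always false for game over, while HideUI removes all widgets.
; Escape and Enter both quit the game.
; NumLock triggers a reset RPC that calls AdminResetGame on BP_GameMode; leftover ghost color-change logic is disconnected.
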(event `self.OnMissionCompleted`
  (params (InstigatorPawn :type "Pawn Object Reference") (bMissionSuccess :type Boolean))
  (bind _returnvalue (`|CreateWidget` "/Game/UI/WBP_GameOver.WBP_GameOver_C" null bMissionSuccess))
  (`UserWidget.AddToViewport` _returnvalue 0))

(event `self.OnGameOver`
  (bind _returnvalue (`|CreateWidget` "/Game/UI/WBP_GameOver.WBP_GameOver_C"))
  (`UserWidget.AddToViewport` _returnvalue 0))

(event `Key|Escape`
  (params (Key :type "Key Structure"))
  (:`Pressed`
    (`KismetSystemLibrary.QuitGame` self "Quit" :!label _label)))

(event `Key|Enter`
  (params (Key :type "Key Structure"))
  (:`Pressed`
    (goto _label)))

(event `HideUI`
  (`WidgetLayoutLibrary.RemoveAllWidgets`))

(event `Key|NumLock`
  (params (Key :type "Key Structure"))
  (:`Pressed`
    (`self.RPC_Reset`)))

(event `RPC_Reset`
  (bind _returnvalue (`GameplayStatics.GetGameMode`))
  (if (`KismetSystemLibrary.IsValid` _returnvalue)
    (bind _asbp_game_mode (cast `/Game/Blueprints/BP_GameMode` _returnvalue))
    (`/Game/Blueprints/BP_GameMode.AdminResetGame` _asbp_game_mode)))

(event `Key|One`
  (params (Key :type "Key Structure")))

(fn `UserConstructionScript`)