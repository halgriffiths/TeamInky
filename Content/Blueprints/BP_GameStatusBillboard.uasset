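; Billboard actor that shows game readiness on a text render component, apparently for a Pacman-versus-ghosts multiplayer game.
; On BeginPlay it queries BP_GameMode for running state and player count, requiring at least three players to be ready.
; The chosen state drives the text and color, though the game-in-progress state has no handler.
; Older win and status message chains, including a delayed re-check, remain disconnected.
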(event `self.ReceiveBeginPlay`
  (`self.DecideBillboard`))

(event `DecideBillboard`
  (`KismetSystemLibrary.PrintString` "DECIDING BILLBOARD")
  (bind _asbp_game_mode (cast `/Game/Blueprints/BP_GameMode` (`GameplayStatics.GetGameMode`))
    (:`then`
      (if (`FPSGameMode.bIsGameRunning` _asbp_game_mode)
        (`self.SetBillboard` "NewEnumerator1")
        (else
          (bind _returnvalue (`GameModeBase.GetNumPlayers` _asbp_game_mode))
          (if (> _returnvalue 2)
            (`self.SetBillboard` "NewEnumerator0")
            (else
              (`self.SetBillboard` "NewEnumerator4"))))))
    (:`CastFailed`
      (`KismetSystemLibrary.PrintString` "CAST FAILED"))))

(event `SetBillboard`
  (params (`Input Enum` :type "/Game/Blueprints/BillboardEnum Enum" :default "NewEnumerator0"))
  (switch `/Game/Blueprints/BillboardEnum` `Input Enum`
    (:`NewEnumerator0`
      (`self.SetTextAndColor` "READY FOR GAME" (make `Color` 0 255 0 255)))
    (:`NewEnumerator4`
      (`self.SetTextAndColor` "NOT ENOUGH PLAYERS" (make `Color` 0 0 255 255)))))

(event `SetTextAndColor`
  (params (Text :type String) (Color :type "Color Structure"))
  (bind _textrender (`self.TextRender`))
  (`TextRenderComponent.K2_SetText` _textrender (`KismetTextLibrary.Conv_StringToText` Text))
  (`TextRenderComponent.SetTextRenderColor` _textrender Color)
  (`KismetSystemLibrary.PrintString` "SET COLOR"))

(fn `UserConstructionScript`)